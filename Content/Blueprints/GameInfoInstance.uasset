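; GameInfoInstance provides the events for hosting and joining multiplayer sessions, judging by its name as the Game Instance.
; HOST_SESSION stores the server name, creates a session from the connection count and LAN flag, then opens Map2 as a listen server on success.
; JOIN_SESSION joins a supplied search result, and both events report success or failure only through printed strings.
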(event `HOST_SESSION`
  (params (PublicConnections :type Integer) (bUseLAN :type Boolean) (ServerName :type String))
  ;[1 1 1] Create session
  (set `self.ServerName` ServerName)
  (`CreateSessionCallbackProxy.CreateSession` (`GameplayStatics.GetPlayerController` 0) PublicConnections bUseLAN
    (:`OnSuccess`
      (`KismetSystemLibrary.PrintString` "Session Created")
      (`GameplayStatics.OpenLevel` "Map2" true "listen"))
    (:`OnFailure`
      (`KismetSystemLibrary.PrintString` "Session Failed"))))

(event `JOIN_SESSION`
  (params (SearchResult :type "BlueprintSessionResult Structure (by ref)"))
  ;[1 1 1] Join Session
  (`JoinSessionCallbackProxy.JoinSession` (`GameplayStatics.GetPlayerController` 0) SearchResult
    (:`OnSuccess`
      (`KismetSystemLibrary.PrintString` "Session Joined"))
    (:`OnFailure`
      (`KismetSystemLibrary.PrintString` "Session Join Fail"))))