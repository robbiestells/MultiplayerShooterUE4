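; Shotgun pickup actor that grants the weapon and starting ammo to an overlapping FirstPersonCharacter.
; On server overlap it adds ammo and marks the gun acquired at GunId, calls PickupGun and copies its FireRate to the character.
; It then disables itself and hides only the root component, without propagating to children, restoring both after a short delay to act as a respawn.
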(event `self.ReceiveActorBeginOverlap`
  (params (OtherActor :type "Actor Object Reference"))
  (if (not (`self.IsDisabled`))
    (`/Engine/EditorBlueprintResources/ActorMacros.Switch Has Authority`
      (:`Authority`
        (bind _asfirst_person_character (cast `/Game/FirstPersonBP/Blueprints/FirstPersonCharacter` OtherActor))
        (bind _gunammos (`/Game/FirstPersonBP/Blueprints/FirstPersonCharacter.GunAmmos` _asfirst_person_character))
        (`KismetArrayLibrary.Array_Set` _gunammos (`self.GunId`) (+ (`|GetArrayItem` _gunammos (`self.GunId`)) (`self.StartingAmmo`)))
        (`KismetArrayLibrary.Array_Set` (`/Game/FirstPersonBP/Blueprints/FirstPersonCharacter.GunsAquired` _asfirst_person_character) (`self.GunId`) true)
        (`/Game/FirstPersonBP/Blueprints/FirstPersonCharacter.PickupGun` _asfirst_person_character (`self.GunId`))
        (set `/Game/FirstPersonBP/Blueprints/FirstPersonCharacter.FireRate` (`self.FireRate`) _asfirst_person_character)
        (set `self.IsDisabled` true)
        (`SceneComponent.SetVisibility` (`self.DefaultSceneRoot`) false false)
        (`KismetSystemLibrary.Delay` 3.0)
        (set `self.IsDisabled` false)
        (`SceneComponent.SetVisibility` (`self.DefaultSceneRoot`) true false)))))

(fn `UserConstructionScript`)